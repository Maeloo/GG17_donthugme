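; Enemy actor that affects the player's vibes by proximity and registers a kill when it hits a FanBox.
; Tick calls AddVibes on the cached FirstPersonCharacter, with a nonzero amount only at close range.
; While the capsule simulates physics, an upward trace detecting a FanBox spawns temporary blood sparks and calls the player's OnKill.
; Attack passes its flag to EnableAttack on the Jill Mixamo anim Blueprint.
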(event `self.ReceiveBeginPlay`
  (bind _outactors (`GameplayStatics.GetAllActorsOfClass` "/Game/FirstPersonBP/Blueprints/FirstPersonCharacter.FirstPersonCharacter_C"))
  (set `self.Player` (`KismetArrayLibrary.Array_Get` _outactors)))

(event `self.ReceiveTick`
  (params (DeltaSeconds :type "Float (single-precision)"))
  (bind _returnvalue (`self.K2_GetActorLocation`))
  (bind _player (`self.Player`))
  (`/Game/FirstPersonBP/Blueprints/FirstPersonCharacter.Add Vibes` _player (`KismetMathLibrary.SelectFloat` 0.05 0.0 (< (`KismetMathLibrary.VSize` (- (`self.K2_GetActorLocation` _player) (`self.K2_GetActorLocation`))) 200.0)))
  (if (`SceneComponent.IsAnySimulatingPhysics` (`self.CapsuleComponent`))
    (bind _outhit (`KismetSystemLibrary.LineTraceSingle` _returnvalue (+ _returnvalue (0.0 0.0 100.0)) "TraceTypeQuery2"))
    (bind (_bblockinghit _binitialoverlap _time _location _impactpoint _normal _impactnormal _physmat _hitactor) (`GameplayStatics.BreakHitResult` _outhit))
    (cast `/Game/BP/FanBox` _hitactor)
    (bind _returnvalue_2 (`GameplayStatics.SpawnEmitterAtLocation` "/Game/StarterContent/Particles/P_BloodSparks.P_BloodSparks" _location))
    (`/Game/FirstPersonBP/Blueprints/FirstPersonCharacter.On Kill` (`self.Player`))
    (`KismetSystemLibrary.Delay` 5.0)
    (`ActorComponent.K2_DestroyComponent` _returnvalue_2)))

(fn `Attack`
  (params (Attack :type Boolean))
  (bind _asmixamo_anim_bp_jill (cast `/Game/MixamoAnimPack/Mixamo_Jill/Anims/MixamoAnimBP_Jill` (`SkeletalMeshComponent.GetAnimInstance` (`self.Mesh`))))
  (set `/Game/MixamoAnimPack/Mixamo_Jill/Anims/MixamoAnimBP_Jill.EnableAttack` Attack _asmixamo_anim_bp_jill))

(fn `UserConstructionScript`)